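; BP_Apple is a falling apple that the player catches with a basket.
; On a hit with an actor tagged Basket, it calls AppleCatched on the BP_PlayerInfo player state and destroys itself.
; Otherwise, a timer started at BeginPlay expires after a short delay, calls MissAppleEvent on the BP_ApplePicker player pawn and destroys the apple, so a miss is decided by lifetime alone.
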(event EventBeginPlay
  (Utilities|FlowControl|Delay 1.2)
  (bind _asbp_apple_picker (Utilities|Casting|CastToBP_ApplePicker (Game|Player|GetPlayerPawn 0)))
  (Default|MissAppleEvent _asbp_apple_picker)
  (Actor|DestroyActor))

(event Collision|EventHit
  (params (MyComp :type Primitive%20Component%20Object%20Reference) (Other :type Actor%20Object%20Reference) (OtherComp :type Primitive%20Component%20Object%20Reference) (bSelfMoved :type Boolean) (HitLocation :type Vector :default "0, 0, 0") (HitNormal :type Vector :default "0, 0, 0") (NormalImpulse :type Vector :default "0, 0, 0") (Hit :type Hit%20Result%20Structure%20%28by%20ref%29))
  (if (Actor|ActorHasTag Other "Basket")
    (bind _asbp_player_info (Utilities|Casting|CastToBP_PlayerInfo (Game|GetPlayerState 0)))
    (Default|AppleCatched _asbp_player_info)
    (Actor|DestroyActor)))

(fn ConstructionScript)