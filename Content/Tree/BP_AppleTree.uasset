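; BP_AppleTree is an apple tree actor that slides along the Y axis and periodically drops apples.
; Each tick moves it by speed and delta time, reversing direction when outside the left/right bounds or on a random roll out of 1000.
; It spawns the apple class at its own transform when a counter passes the spawn threshold; the counter grows by a fixed per-tick step, making spawn rate frame-rate dependent.
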(event EventTick
  (params (DeltaSeconds :type Float%20%28single-precision%29))
  (CallFunction|MoveTree DeltaSeconds)
  (CallFunction|SpawnApple))

(fn ConstructionScript)

(fn MoveTree
  (params (DeltaTime :type Float%20%28double-precision%29))
  (bind _returnvalue (Transformation|GetActorLocation))
  (Transformation|SetActorLocation (Math|Vector|MakeVector (.x _returnvalue) (+ (.y _returnvalue) (* (Variables|Default|GetSpeed) DeltaTime (.y (Variables|Default|GetDirection)))) (.z _returnvalue)) false false)
  (bind _isoutofbound (CallFunction|IsOutOfBound))
  (if (or _isoutofbound (< (Math|Random|RandomInteger 1000) (Variables|Default|GetPercentageToChangeDirRandomly)))
    (Variables|Default|SetDirection (Math|Vector|MakeVector 0.0 (* (.y (Variables|Default|GetDirection)) -1.0) 0.0))))

(fn IsOutOfBound
  (bind _returnvalue (Transformation|GetActorLocation))
  (return (or (> (.y _returnvalue) (Variables|Default|GetLeftBoundY)) (< (.y _returnvalue) (Variables|Default|GetRightBoundY)))))

(fn SpawnApple
  (if (> (Variables|Default|GetTimeBeforeSpawning) (Variables|Default|GetTimeToSpawn))
    (Game|SpawnActorfromClass (Variables|Default|GetApplePrefab) (Transformation|GetActorTransform) "Undefined" "MultiplyWithRoot" 0 0)
    (Variables|Default|SetTimeBeforeSpawning 0.0)
    (else
      (Variables|Default|SetTimeBeforeSpawning (+ (Variables|Default|GetTimeBeforeSpawning) 0.01)))))