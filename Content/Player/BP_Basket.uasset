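; BP_Basket is a player basket actor that slides along the Y axis according to the horizontal mouse position.
; Tick calls MoveBaskets, which keeps X and Z and sets Y from cursor X minus a hardcoded center offset, negated and scaled by Speed and delta time.
; That product becomes the absolute Y rather than an increment, so the basket's position varies with frame time.
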(event EventBeginPlay)

(event Collision|EventActorBeginOverlap
  (params (OtherActor :type Actor%20Object%20Reference)))

(event EventTick
  (params (DeltaSeconds :type Float%20%28single-precision%29))
  (CallFunction|MoveBaskets DeltaSeconds))

(fn ConstructionScript)

(fn MoveBaskets
  (params (DeltaTime :type Float%20%28double-precision%29))
  (bind _returnvalue (Transformation|GetActorLocation))
  (Variables|Default|SetDeltaTime DeltaTime)
  (Transformation|SetActorLocation (Math|Vector|MakeVector (.x _returnvalue) (* (- (.LocationX (Game|Player|GetMousePosition (Game|GetPlayerController 0))) 7e+02) (Variables|Default|GetDeltaTime) (Variables|Default|GetSpeed) -1.0) (.z _returnvalue)) false false))