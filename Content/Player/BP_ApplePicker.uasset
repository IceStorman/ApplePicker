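; Player blueprint for an Apple Picker game that controls a set of baskets and tracks remaining health.
; BeginPlay registers the input mapping, creates the canvas widget and initializes the baskets.
; IA_Move shifts every valid basket along the Y axis, scaled by Speed and inverted.
; MissAppleEvent destroys the basket indexed by Health, decrements Health, plays sounds, and reloads the current level when Health runs out.
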(event Custom|MissAppleEvent
  (Actor|DestroyActor (Utilities|Array|Get(acopy) (Variables|Default|Getbaskets) (- (Variables|Default|GetHealth) 1)))
  (Math|Integer|DecrementInt (Variables|Default|GetHealth)
    (:%20%20
      (Class|SoundSubsystem|PlaySound (Subsystems|GetSoundSubsystem) "AppleLost")
      (if (<= (Variables|Default|GetHealth) 0)
        (Class|SoundSubsystem|PlaySound (Subsystems|GetSoundSubsystem) "GameOver")
        (bind _returnvalue (Game|GetCurrentLevelName true))
        (Game|OpenLevel(byName) (Utilities|String|StringToName _returnvalue))))))

(event Input|EnhancedActionEvents|EnhancedInputActionIA_Move
  (params (ActionValue :type Float%20%28double-precision%29) (ElapsedSeconds :type Float%20%28double-precision%29) (TriggeredSeconds :type Float%20%28double-precision%29) (InputAction :type Input%20Action%20Object%20Reference :default "/Game/Player/IA_Move.IA_Move"))
  (for _array_element (Variables|Default|Getbaskets)
    (Utilities|IsValid _array_element
      (:Is%20Valid
        (Transformation|SetActorLocation _array_element (Math|Vector|MakeVector (.x (Transformation|GetActorLocation _array_element)) (+ (.y (Transformation|GetActorLocation _array_element)) (* ActionValue (Variables|Default|Getspeed) -1.0)) (.z (Transformation|GetActorLocation _array_element))) false false)))))

(event EventBeginPlay
  (Input|AddMappingContext (PlayerController|LocalPlayerSubsystems|GetEnhancedInputLocalPlayerSubsystem (Game|GetPlayerController 0)) "/Game/Player/IMC_Default.IMC_Default" 0 "(bIgnoreAllPressedKeysUntilRelease=True,bForceImmediately=False,bNotifyUserSettings=False)")
  (bind _returnvalue (UserInterface|CreateWidget "/Game/Player/UI/WBP_Canvas.WBP_Canvas_C"))
  (UserInterface|Viewport|AddtoViewport _returnvalue 0)
  (Class|ApplePicker|InitBaskets))

(fn ConstructionScript)